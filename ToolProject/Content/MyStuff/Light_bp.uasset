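; Light Blueprint for a bulb fixture with optional random color and intensity, and chance-based flickering.
; The construction script applies intensity, then picks one of five colors or LightColor; only some branches reach the intensity randomization, after it is applied.
; BeginPlay gives the bulb a dynamic material with random color and emissive values, independent of the light color.
; Random rolls above FlickerBulbChance start a timeline flickering light and material, replaying after random delays.
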(event `SetBulbColor`
  (bind _bulbmaterialinstance (`self.BulbMaterialInstance`))
  (bind _linearcolor (make `LinearColor` (`KismetMathLibrary.RandomFloatInRange` 0.0 255.0) (`KismetMathLibrary.RandomFloatInRange` 0.0 255.0) (`KismetMathLibrary.RandomFloatInRange` 0.0 255.0)))
  ;[1 1 1] Comment
  (`MaterialInstanceDynamic.SetVectorParameterValue` _bulbmaterialinstance "BulbColor" _linearcolor)
  (`MaterialInstanceDynamic.SetVectorParameterValue` _bulbmaterialinstance "EmissiveColor" _linearcolor)
  (`MaterialInstanceDynamic.SetScalarParameterValue` _bulbmaterialinstance "EmissiveInt" (`KismetMathLibrary.RandomFloatInRange` 0.0 1.0)))

(event `self.ReceiveBeginPlay`
  (bind _returnvalue (`KismetMaterialLibrary.CreateDynamicMaterialInstance` (`PrimitiveComponent.GetMaterial` (`self.BulbMesh`) 0)))
  (bind _output_get (set `self.BulbMaterialInstance` _returnvalue))
  (`PrimitiveComponent.SetMaterial` (`self.BulbMesh`) 0 _output_get)
  (`self.RandomizeFlickering`)
  (`self.SetBulbColor`))

(event `RandomizeFlickering`
  (`/Engine/EditorBlueprintResources/StandardMacros.CompareFloat` (`KismetMathLibrary.RandomFloatInRange` 0.0 1.0) (`self.FlickerBulbChance`)
    (:`>`
      (set `self.IsFlickerLight?` true))
    (:`==`
      (set `self.IsFlickerLight?` false))
    (:`<`
      (set `self.IsFlickerLight?` false)))
  (if (`self.IsFlickerLight?`)
    (`KismetSystemLibrary.Delay` (`KismetMathLibrary.RandomFloatInRange` 2.0 5.0))
    (`self.StartFlickering`)))

(event `StartFlickering`
  (bind (_direction _flickertrack1) (`Timeline|Flicker` :!via `PlayFromStart`)
    (:`Update`
      (`LightComponent.SetIntensity` (`self.Light`) (* _flickertrack1 (`self.Intensity`)))
      (`MaterialInstanceDynamic.SetScalarParameterValue` (`self.BulbMaterialInstance`) "BulbIntensity" _flickertrack1))
    (:`Finished`
      (`KismetSystemLibrary.Delay` (`KismetMathLibrary.RandomFloatInRange` 2.0 10.0))
      (`self.StartFlickering`))))

(fn `UserConstructionScript`
  (locals (NewLocalVar_0 :type Boolean :default true))
  (bind _light (`self.Light`))
  (`LightComponent.SetIntensity` _light (`self.Intensity`))
  (if (`self.RandomizedLightColor?`)
    (switch `int` (`KismetMathLibrary.RandomIntegerInRange` 0 4)
      (:`0`
        (`LightComponent.SetLightColor` _light (`KismetMathLibrary.Conv_ColorToLinearColor` (make `Color` 255 0 0 1)) true))
      (:`1`
        (`LightComponent.SetLightColor` _light (`KismetMathLibrary.Conv_ColorToLinearColor` (make `Color` 0 255 255)) true))
      (:`2`
        (`LightComponent.SetLightColor` _light (`KismetMathLibrary.Conv_ColorToLinearColor` (make `Color` 0 0 255)) true)
        (if (`self.RandomizedLightInt?`) :!label _label
          (set `self.Intensity` (`KismetMathLibrary.RandomFloatInRange` 2500.0 5000.0))))
      (:`3`
        (`LightComponent.SetLightColor` _light (`KismetMathLibrary.Conv_ColorToLinearColor` (make `Color` 0 255)) true)
        (goto _label))
      (:`4`
        (`LightComponent.SetLightColor` _light (`KismetMathLibrary.Conv_ColorToLinearColor` (make `Color` 255 0 255)) true)
        (goto _label)))
    (else
      (`LightComponent.SetLightColor` _light (`self.Light Color`) true)
      (goto _label))))