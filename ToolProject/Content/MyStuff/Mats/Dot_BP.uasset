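; Dot actor, a sphere that gets a randomized look when play begins and destroys itself when something overlaps it.
; BeginPlay creates a dynamic instance of ExampleMat with random color, emissive color, emissive intensity and roughness, drawing color channels from 0–255 rather than 0–1.
; Disconnected nodes that never run sketch a random rarity roll filling a Pokemon struct with rarity and attack power.
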(event `self.ReceiveBeginPlay`
  (bind _linearcolor (make `LinearColor` (`KismetMathLibrary.RandomFloatInRange` 0.0 255.0) (`KismetMathLibrary.RandomFloatInRange` 0.0 255.0) (`KismetMathLibrary.RandomFloatInRange` 0.0 255.0)))
  (bind _returnvalue (`PrimitiveComponent.CreateDynamicMaterialInstance` (`self.Sphere`) 0 "/Game/MyStuff/Mats/ExampleMat.ExampleMat" "None"))
  (`MaterialInstanceDynamic.SetVectorParameterValue` _returnvalue "Color" _linearcolor)
  (`MaterialInstanceDynamic.SetVectorParameterValue` _returnvalue "EmissiveColor" _linearcolor)
  (`MaterialInstanceDynamic.SetScalarParameterValue` _returnvalue "EmissiveInt" (`KismetMathLibrary.RandomFloatInRange` 0.0 1.0))
  (`MaterialInstanceDynamic.SetScalarParameterValue` _returnvalue "Roughness" (`KismetMathLibrary.RandomFloatInRange` 0.0 1.0)))

(event `self.Sphere.OnComponentBeginOverlap`
  (params (OverlappedComponent :type "PrimitiveComponent Object Reference") (OtherActor :type "Actor Object Reference") (OtherComp :type "PrimitiveComponent Object Reference") (OtherBodyIndex :type Integer) (bFromSweep :type Boolean) (SweepResult :type "HitResult Structure (by ref)"))
  (`self.K2_DestroyActor`))

(fn `UserConstructionScript`)